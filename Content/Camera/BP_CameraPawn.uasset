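; Camera pawn that spawns a BP_moving_object at BeginPlay and follows it each tick.
; The 3d flag on the KalmanMod game mode selects the view.
; In 3D, the camera takes an offset, scaled position derived from the object's location and rotates to look at it.
; Otherwise, it tracks the object's X and Y at the stored camera height without updating rotation.
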(event EventBeginPlay
  (bind _askalman_mod (Utilities|Casting|CastToKalmanMod (Game|GetGameMode)))
  (Variables|Default|SetAs%20Kalman%20Mod _askalman_mod)
  (bind _returnvalue (Game|SpawnActorfromClass "/Game/Moving_object/BP_moving_object.BP_moving_object_C" (Variables|Default|GetSpawn%20Transform) "Undefined" 0 0))
  (Variables|Default|Setobject_ref _returnvalue)
  (Transformation|SetWorldLocation (Variables|Default|GetCamera) (Math|Vector|MakeVector (.x (Transformation|GetWorldLocation (Variables|/Game/Moving_object/BP_moving_object.BP_moving_object_C|GetObject (Variables|Default|Getobject_ref)))) (.y (Transformation|GetWorldLocation (Variables|/Game/Moving_object/BP_moving_object.BP_moving_object_C|GetObject (Variables|Default|Getobject_ref)))) (Variables|Default|GetCameraLocation%20Z)) false false)
  (bind _askalman_mod_2 (Utilities|Casting|CastToKalmanMod (Game|GetGameMode)))
  (Variables|Default|SetKalman%20Mod%20ref _askalman_mod_2))

(event Collision|EventActorBeginOverlap
  (params (OtherActor :type Actor%20Object%20Reference)))

(event EventTick
  (params (DeltaSeconds :type Float%20%28single-precision%29))
  (bind _object_ref (Variables|Default|Getobject_ref))
  (bind _object_ref_2 (Variables|Default|Getobject_ref))
  (bind _object (Variables|/Game/Moving_object/BP_moving_object.BP_moving_object_C|GetObject _object_ref))
  (bind _object_2 (Variables|/Game/Moving_object/BP_moving_object.BP_moving_object_C|GetObject _object_ref_2))
  (bind _returnvalue (Transformation|GetWorldLocation _object))
  (bind _returnvalue_2 (Transformation|GetWorldLocation _object_2))
  (if (Variables|/Game/GameMod/KalmanMod.KalmanMod_C|Get3d (Variables|Default|GetAs%20Kalman%20Mod))
    (Variables|Default|SetCameraLocation%20Z 1e+03)
    (Transformation|SetWorldLocation (Variables|Default|GetCamera) (Math|Vector|MakeVector (* (.x _returnvalue_2) 0.8) (* (+ (.y _returnvalue_2) -5e+02) 0.9) (* (+ (Variables|Default|GetCameraLocation%20Z) (.z _returnvalue_2)) 0.5)) false false)
    (Transformation|SetWorldRotation (Variables|Default|GetCamera) (Math|Rotator|FindLookatRotation (Transformation|GetWorldLocation (Variables|Default|GetCamera)) (Transformation|GetWorldLocation (Variables|/Game/Moving_object/BP_moving_object.BP_moving_object_C|GetObject (Variables|Default|Getobject_ref)))) false false)
    (else
      (Transformation|SetWorldLocation (Variables|Default|GetCamera) (Math|Vector|MakeVector (.x _returnvalue) (.y _returnvalue) (Variables|Default|GetCameraLocation%20Z)) false false))))

(fn ConstructionScript)