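; BP_moving_object is a moving object that flies a scripted test trajectory, in 2D or 3D as set by the KalmanMod game mode.
; BeginPlay calls RandomBoost at delayed intervals, stepping a sequential MultiGate through initial acceleration, two maneuvers chosen by test number, and a stop.
; Timelines blend heading and acceleration, which v=v0+a·t converts into ProjectileMovement velocity.
; In 3D, Tick also turns Object toward the camera and syncs Object1's XY position.
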(event Custom|RandomBoost
  ;[1 1 1 0.1] Boost Logic
  ;;[1 1 1 0.2] Test(1.2.3)
  (Utilities|FlowControl|MultiGate false false 0
    (:Out%200
      (bind _newtrack_0 (Timeline|Timeline_0 PlayFromStart)
        (:Update
          (bind _output_get (Variables|Default|SetAlpha 45.0))
          (bind _output_get_2 (Variables|Default|SetBoostPower (Math|Float|Lerp 2e+01 35.0 _newtrack_0)))
          (if (!= (Variables|/Game/GameMod/KalmanMod.KalmanMod_C|Get3d (Variables|Default|GetKalman%20Mod%20ref)) true)
            ;;[1 1 1 0.1] v=v0+a*t
            (bind _time (Timeline|Time PlayFromStart)
              (:Update
                (bind _output_get_3 (Variables|Default|SetNewToAxes (Math|Vector|MakeVector (+ (.x (Variables|Default|GetOldToAxes)) (* _time (* (Variables|Default|GetBoostPower) (Math|Trig|Cos(Degrees) (Variables|Default|GetAlpha))))) (+ (.y (Variables|Default|GetOldToAxes)) (* _time (* (Variables|Default|GetBoostPower) (Math|Trig|Sin(Degrees) (Variables|Default|GetAlpha))))) (+ (.z (Variables|Default|GetOldToAxes)) (* _time (Variables|Default|GetBoostPower_Z))))))
                (Game|Components|ProjectileMovement|SetVelocityinLocalSpace (Variables|Default|GetProjectileMovement) (Math|Vector|MakeVector (.x _output_get_3) (.y _output_get_3) (.z _output_get_3))))
              (:Finished
                (Variables|Default|SetOldToAxes (Variables|Default|GetNewToAxes))))
            (else
              (bind _output_get_4 (Variables|Default|SetBoostPower_Z (Math|Float|Lerp 0.0 12.0 _newtrack_0)))
              (Timeline|Time PlayFromStart))))))
    (:Out%201
      (bind _newtrack_0_2 (Timeline|Timeline_1 PlayFromStart)
        (:Update
          (Utilities|RoadMacro
            (:then
              (bind _output_get_5 (Variables|Default|SetAlpha (Math|Float|Lerp _output_get 1.8e+02 _newtrack_0_2)))
              (bind _output_get_6 (Variables|Default|SetBoostPower (Math|Float|Lerp _output_get_2 4e+01 _newtrack_0_2)))
              (if (!= (Variables|/Game/GameMod/KalmanMod.KalmanMod_C|Get3d (Variables|Default|GetKalman%20Mod%20ref)) true)
                (Timeline|Time PlayFromStart)
                (else
                  (bind _output_get_7 (Variables|Default|SetBoostPower_Z (Math|Float|Lerp _output_get_4 -1e+01 _newtrack_0_2)))
                  (Timeline|Time PlayFromStart))))
            (:then2
              (bind _output_get_8 (Variables|Default|SetAlpha (Math|Float|Lerp _output_get 2.2e+02 _newtrack_0_2)))
              (bind _output_get_9 (Variables|Default|SetBoostPower (Math|Float|Lerp _output_get_2 9e+01 _newtrack_0_2)))
              (if (!= (Variables|/Game/GameMod/KalmanMod.KalmanMod_C|Get3d (Variables|Default|GetKalman%20Mod%20ref)) true)
                (Timeline|Time PlayFromStart)
                (else
                  (bind _output_get_10 (Variables|Default|SetBoostPower_Z (Math|Float|Lerp _output_get_4 -25.0 _newtrack_0_2)))
                  (Timeline|Time PlayFromStart))))
            (:then3
              (bind _output_get_11 (Variables|Default|SetAlpha (Math|Float|Lerp _output_get 1.8e+02 _newtrack_0_2)))
              (bind _output_get_12 (Variables|Default|SetBoostPower (Math|Float|Lerp _output_get_2 4e+01 _newtrack_0_2)))
              (if (!= (Variables|/Game/GameMod/KalmanMod.KalmanMod_C|Get3d (Variables|Default|GetKalman%20Mod%20ref)) true)
                (Timeline|Time PlayFromStart)
                (else
                  (bind _output_get_13 (Variables|Default|SetBoostPower_Z (Math|Float|Lerp _output_get_4 -1e+01 _newtrack_0_2)))
                  (Timeline|Time PlayFromStart))))))))
    (:Out%202
      (bind _newtrack_0_3 (Timeline|Timeline_2 PlayFromStart)
        (:Update
          (Utilities|RoadMacro
            (:then
              (Variables|Default|SetAlpha (Math|Float|Lerp _output_get_5 2.9e+02 _newtrack_0_3))
              (Variables|Default|SetBoostPower (Math|Float|Lerp _output_get_6 5e+01 _newtrack_0_3))
              (if (!= (Variables|/Game/GameMod/KalmanMod.KalmanMod_C|Get3d (Variables|Default|GetKalman%20Mod%20ref)) true)
                (Timeline|Time PlayFromStart)
                (else
                  (Variables|Default|SetBoostPower_Z (Math|Float|Lerp _output_get_7 -2e+01 _newtrack_0_3))
                  (Timeline|Time PlayFromStart))))
            (:then2
              (Variables|Default|SetAlpha (Math|Float|Lerp _output_get_8 45.0 _newtrack_0_3))
              (Variables|Default|SetBoostPower (Math|Float|Lerp _output_get_9 1e+02 _newtrack_0_3))
              (if (!= (Variables|/Game/GameMod/KalmanMod.KalmanMod_C|Get3d (Variables|Default|GetKalman%20Mod%20ref)) true)
                (Timeline|Time PlayFromStart)
                (else
                  (Variables|Default|SetBoostPower_Z (Math|Float|Lerp _output_get_10 2e+01 _newtrack_0_3))
                  (Timeline|Time PlayFromStart))))
            (:then3
              (Variables|Default|SetAlpha (Math|Float|Lerp _output_get_11 0.0 _newtrack_0_3))
              (Variables|Default|SetBoostPower (Math|Float|Lerp _output_get_12 5e+01 _newtrack_0_3))
              (if (!= (Variables|/Game/GameMod/KalmanMod.KalmanMod_C|Get3d (Variables|Default|GetKalman%20Mod%20ref)) true)
                (Timeline|Time PlayFromStart)
                (else
                  (Variables|Default|SetBoostPower_Z (Math|Float|Lerp _output_get_13 -1e+01 _newtrack_0_3))
                  (Timeline|Time PlayFromStart))))))))
    (:Out%203
      (bind _stop_track (Timeline|Stop PlayFromStart)
        (:Update
          (Game|Components|ProjectileMovement|SetVelocityinLocalSpace (Variables|Default|GetProjectileMovement) (Math|Vector|MakeVector (Math|Float|Lerp 0.0 (.x (Variables|Default|GetOldToAxes)) _stop_track) (Math|Float|Lerp 0.0 (.y (Variables|Default|GetOldToAxes)) _stop_track) (Math|Float|Lerp 0.0 (.z (Variables|Default|GetOldToAxes)) _stop_track))))))))

(event EventBeginPlay
  (bind _askalman_mod (Utilities|Casting|CastToKalmanMod (Game|GetGameMode)))
  (Variables|Default|SetKalman%20Mod%20ref _askalman_mod)
  (bind _returnvalue (Actor|GetActorOfClass "/Game/Camera/BP_CameraPawn.BP_CameraPawn_C"))
  (Variables|Default|SetAs_Camera _returnvalue)
  (Utilities|ForceMacro)
  (Utilities|ForceMacro)
  (Utilities|ForceMacro)
  (CallFunction|RandomBoost))

(event EventTick
  (params (DeltaSeconds :type Float%20%28single-precision%29))
  (bind _object (Variables|Default|GetObject))
  (bind _object_2 (Variables|Default|GetObject))
  (bind _as_camera (Variables|Default|GetAs_Camera))
  (bind _returnvalue (Transformation|GetWorldLocation _object))
  (bind _returnvalue_2 (Transformation|GetWorldLocation _object_2))
  (bind _camera (Variables|/Game/Camera/BP_CameraPawn.BP_CameraPawn_C|GetCamera _as_camera))
  (bind _returnvalue_3 (Transformation|GetWorldLocation _camera))
  (bind _returnvalue_4 (Math|Rotator|FindLookatRotation _returnvalue _returnvalue_3))
  (Utilities|FlowControl|Delay 0.1)
  (if (Variables|/Game/GameMod/KalmanMod.KalmanMod_C|Get3d (Variables|Default|GetKalman%20Mod%20ref))
    (Transformation|SetWorldRotation (Variables|Default|GetObject) (Math|Rotator|MakeRotator (.roll _returnvalue_4) (+ (.pitch _returnvalue_4) 9e+01) (.yaw _returnvalue_4)) false false)
    (Transformation|SetWorldLocation (Variables|Default|GetObject1) (Math|Vector|MakeVector (.x _returnvalue_2) (.y _returnvalue_2) 0.0) false false)))

(fn ConstructionScript)